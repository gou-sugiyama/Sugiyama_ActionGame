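; Enemy character Blueprint that attacks the player with a sword and dies when its HP runs out.
; On BeginPlay it binds the child-actor sword's collision overlap, dealing damage to ThirdPersonCharacter through a DoOnce that SlashAttack resets before playing the slash montage, limiting each swing to one hit.
; AnyDamage reduces HP; at zero it disables movement, ragdolls the mesh and destroys the actor after a short delay.
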(event `self.ReceiveBeginPlay`
  (bind _asbase_weapon_sword_1 (cast `/Game/ThirdPersonBP/Blueprints/BaseWeapon_Sword1` (`ChildActorComponent.ChildActor` (`self.ChildActor`))))
  (add `PrimitiveComponent.OnComponentBeginOverlap` (`/Game/ThirdPersonBP/Blueprints/BaseWeapon.SwordCollision` _asbase_weapon_sword_1) (delegate `OnSwordCollisionBeginOverlap`)))

(event `OnSwordCollisionBeginOverlap`
  (params (OverlappedComponent :type "PrimitiveComponent Object Reference") (OtherActor :type "Actor Object Reference") (OtherComp :type "PrimitiveComponent Object Reference") (OtherBodyIndex :type Integer) (bFromSweep :type Boolean) (SweepResult :type "HitResult Structure (by ref)"))
  (bind _asthird_person_character (cast `/Game/ThirdPersonBP/Blueprints/ThirdPersonCharacter` OtherActor))
  (`/Engine/EditorBlueprintResources/StandardMacros.DoOnce` false :!label _label
    (:`Completed`
      (`GameplayStatics.ApplyDamage` _asthird_person_character 2.0))))

(event `SlashAttack`
  (`|ExecutionSequence`
    (:`then_0`
      (goto _label :!via `Reset`))
    (:`then_1`
      (`self.PlayAnimMontage` "/Game/Enemy_Sword_And_Shield_Slash_Anim_mixamo_com_Montage.Enemy_Sword_And_Shield_Slash_Anim_mixamo_com_Montage"))))

(event `self.ReceiveAnyDamage`
  (params (Damage :type "Float (single-precision)") (DamageType :type "DamageType Object Reference") (InstigatedBy :type "Controller Object Reference") (DamageCauser :type "Actor Object Reference"))
  (bind _mesh (`self.Mesh`))
  (bind _output_get (set `self.HP` (- (`self.HP`) Damage)))
  (if (<= _output_get 0.0)
    (`CharacterMovementComponent.DisableMovement` (`self.CharacterMovement`))
    (`PrimitiveComponent.SetCollisionEnabled` _mesh "PhysicsOnly")
    (`SkeletalMeshComponent.SetAllBodiesSimulatePhysics` _mesh true)
    (`KismetSystemLibrary.Delay` 3.0)
    (`self.K2_DestroyActor`)))

(fn `UserConstructionScript`)